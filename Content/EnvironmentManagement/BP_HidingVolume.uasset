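; BP_HidingVolume is a trigger volume that marks the player as hidden while they stand inside it.
; Its TriggerBox overlap claims the volume for one Character at a time, tracked by InUse and CharacterInVolume, and any Character leaving clears it.
; For Player-tagged characters, it adds or removes the CharacterStates.Hidden gameplay tag and prints debug text.
; On BeginPlay it caches trackers from EnvironmentController, unused in these graphs.
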(event `self.ReceiveBeginPlay`
  (bind _trackers (`/Game/EnvironmentManagement/C_EnvironmentController.ReturnAllTrackers` (`self.EnvironmentController`)))
  (set `self.All Trackers` _trackers))

(event `self.TriggerBox.OnComponentBeginOverlap`
  (params (OverlappedComponent :type "PrimitiveComponent Object Reference") (OtherActor :type "Actor Object Reference") (OtherComp :type "PrimitiveComponent Object Reference") (OtherBodyIndex :type Integer) (bFromSweep :type Boolean) (SweepResult :type "HitResult Structure (by ref)"))
  (if (not (`self.InUse`))
    (bind _ascharacter (cast `Character` OtherActor))
    (set `self.CharacterInVolume` _ascharacter)
    (set `self.InUse` true)
    (if (`self.ActorHasTag` OtherActor "Player")
      (bind _asbp_first_person_character (cast `/Game/FirstPerson/Blueprints/BP_FirstPersonCharacter` OtherActor))
      (`BlueprintGameplayTagLibrary.AddGameplayTag` (`/Game/FirstPerson/Blueprints/BP_FirstPersonCharacter.CharacterStates` _asbp_first_person_character) (struct :`TagName` "CharacterStates.Hidden"))
      (`KismetSystemLibrary.PrintString` "Player is hiding" true true (struct :`G` 1.0 :`B` 0.030778 :`A` 1.0)))))

(event `self.TriggerBox.OnComponentEndOverlap`
  (params (OverlappedComponent :type "PrimitiveComponent Object Reference") (OtherActor :type "Actor Object Reference") (OtherComp :type "PrimitiveComponent Object Reference") (OtherBodyIndex :type Integer))
  (if (`self.InUse`)
    (cast `Character` OtherActor)
    (set `self.CharacterInVolume` null)
    (set `self.InUse` false)
    (if (`self.ActorHasTag` OtherActor "Player")
      (bind _asbp_first_person_character (cast `/Game/FirstPerson/Blueprints/BP_FirstPersonCharacter` OtherActor))
      (`BlueprintGameplayTagLibrary.RemoveGameplayTag` (`/Game/FirstPerson/Blueprints/BP_FirstPersonCharacter.CharacterStates` _asbp_first_person_character) (struct :`TagName` "CharacterStates.Hidden"))
      (`KismetSystemLibrary.PrintString` "Player stopped hiding" true true (struct :`G` 1.0 :`B` 0.030778 :`A` 1.0)))))

(fn `UserConstructionScript`)