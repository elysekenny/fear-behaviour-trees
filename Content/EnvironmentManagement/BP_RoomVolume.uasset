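; BP_RoomVolume is a trigger volume that tracks which characters occupy the room identified by its RoomID.
; On BeginPlay it gets all trackers from CEnvironmentController and binds ReturnCharacters to each.
; Overlaps maintain CharactersInRoom, and each entry also notifies every tracker through CharacterEnterRoom.
; ReturnCharacters reads the BeginPlay loop's element, setting its EnemyCurrentRoom to RoomID if its owner is inside.
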(event `self.ReceiveBeginPlay`
  (bind _trackers (`/Game/EnvironmentManagement/C_EnvironmentController.ReturnAllTrackers` (`self.C_EnvironmentController`)))
  (bind _output_get (set `self.Tracker References` _trackers))
  (for _array_element _output_get
    (add `/Game/AI/Components/C_InformationTracker.ReturnCharactersInRoom` _array_element (delegate `Return Characters`))))

(event `Return Characters`
  (bind _ascharacter (cast `Character` (`ActorComponent.GetOwner` (stale `self.ReceiveBeginPlay` _array_element))))
  (if (`KismetArrayLibrary.Array_Contains` (`self.CharactersInRoom`) _ascharacter)
    (set `/Game/AI/Components/C_InformationTracker.EnemyCurrentRoom` (`self.RoomID`) (stale `self.ReceiveBeginPlay` _array_element))))

(event `self.TriggerBox.OnComponentBeginOverlap`
  (params (OverlappedComponent :type "PrimitiveComponent Object Reference") (OtherActor :type "Actor Object Reference") (OtherComp :type "PrimitiveComponent Object Reference") (OtherBodyIndex :type Integer) (bFromSweep :type Boolean) (SweepResult :type "HitResult Structure (by ref)"))
  (bind _ascharacter (cast `Character` OtherActor))
  (`KismetArrayLibrary.Array_Add` (`self.CharactersInRoom`) _ascharacter)
  (for _array_element (`self.Tracker References`)
    (`/Game/AI/Components/C_InformationTracker.Character Enter Room` _array_element (`self.RoomID`) _ascharacter)))

(event `self.TriggerBox.OnComponentEndOverlap`
  (params (OverlappedComponent :type "PrimitiveComponent Object Reference") (OtherActor :type "Actor Object Reference") (OtherComp :type "PrimitiveComponent Object Reference") (OtherBodyIndex :type Integer))
  (bind _ascharacter (cast `Character` OtherActor))
  (`KismetArrayLibrary.Array_RemoveItem` (`self.CharactersInRoom`) _ascharacter))

(fn `UserConstructionScript`)